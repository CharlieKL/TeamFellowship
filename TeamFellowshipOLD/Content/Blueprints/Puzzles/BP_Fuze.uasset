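; BP_Fuze is a puzzle fuse piece that rotates a quarter turn each time it is interacted with.
; PossibleInteraction plays a timeline that lerps the Fuze component's pitch by 90 degrees, then saves the new pitch, ignoring further interactions while rotating.
; The construction script shows or hides the Top, Right, Left and Bottom components from per-side booleans, so each instance sets its own layout.
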(event `/Game/InteractableObjects/Interfaces/Interact.PossibleInteraction`
  (bind _savedpitch (`self.SavedPitch`))
  (bind _returnvalue (+ _savedpitch 90.0))
  (if (not (`self.IsRotating`))
    (set `self.IsRotating` true)
    (bind (_direction _newtrack_0) (`Timeline|Timeline_0` :!via `PlayFromStart`)
      (:`Update`
        (`SceneComponent.K2_SetRelativeRotation` (`self.Fuze`) (`KismetMathLibrary.RLerp` (`KismetMathLibrary.MakeRotator` 0.0 _savedpitch) (`KismetMathLibrary.MakeRotator` 0.0 _returnvalue) _newtrack_0) false false))
      (:`Finished`
        (set `self.SavedPitch` _returnvalue)
        (set `self.IsRotating` false)))))

(fn `BottomVisibility`
  (bind _bottom (`self.Bottom`))
  (if (`self.BottomVis`)
    (`SceneComponent.SetVisibility` _bottom true false)
    (else
      (`SceneComponent.SetVisibility` _bottom false false))))

(fn `LeftVisibility`
  (bind _left (`self.Left`))
  (if (`self.LeftVis`)
    (`SceneComponent.SetVisibility` _left true false)
    (else
      (`SceneComponent.SetVisibility` _left false false))))

(fn `RightVisibility`
  (bind _right (`self.Right`))
  (if (`self.RightVis`)
    (`SceneComponent.SetVisibility` _right true false)
    (else
      (`SceneComponent.SetVisibility` _right false false))))

(fn `TopVisibility`
  (if (`self.TopVis`)
    (`SceneComponent.SetVisibility` (`self.Top`) true false)
    (else
      (`SceneComponent.SetVisibility` (`self.Top`) false false))))

(fn `UserConstructionScript`
  (`self.TopVisibility`)
  (`self.RightVisibility`)
  (`self.LeftVisibility`)
  (`self.BottomVisibility`))