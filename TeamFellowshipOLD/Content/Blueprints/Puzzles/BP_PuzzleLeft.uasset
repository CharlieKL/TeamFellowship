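; BP_PuzzleLeft is the left element of a rotation puzzle linked to a bookcase door.
; On BeginPlay it casts DoorFromLevel to BP_Bookcase and caches the reference.
; Correct and incorrect direction events report to the bookcase through LeftDone and LeftUndone.
; Toggle events write the bookcase's rotation flags, passing the input through for CanRotateLeft but always setting CanRotateRight to false.
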(event `self.ReceiveBeginPlay`
  (bind _asbp_bookcase (cast `/Game/Blueprints/BP_Bookcase` (`self.Door_FromLevel`)))
  (set `self.BookcaseRef` _asbp_bookcase))

(event `CorrectDirection`
  (`/Game/Blueprints/BP_Bookcase.LeftDone` (`self.BookcaseRef`)))

(event `IncorrectDirection`
  (`/Game/Blueprints/BP_Bookcase.LeftUndone` (`self.BookcaseRef`)))

(event `ToggleCanRotateLeft`
  (params (Bool :type Boolean))
  (set `/Game/Blueprints/BP_Bookcase.CanRotateLeft` Bool (`self.BookcaseRef`)))

(event `ToggleCanRotateRight`
  (set `/Game/Blueprints/BP_Bookcase.CanRotateRight` false (`self.BookcaseRef`)))

(fn `UserConstructionScript`)