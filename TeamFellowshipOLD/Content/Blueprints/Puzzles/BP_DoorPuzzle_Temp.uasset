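; BP_DoorPuzzle_Temp is a temporary puzzle door actor that removes itself once both a left and a right part are solved.
; Events for left and right completion or undo set two flags, LeftCorrect and RightCorrect.
; When either side finishes while the other is already correct, it clears CanRotate and destroys the actor.
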(event `LeftDone`
  (set `self.LeftCorrect` true)
  (if (`self.RightCorrect`)
    (set `self.CanRotate?` false :!label _label)
    (`self.K2_DestroyActor`)))

(event `LeftUnDone`
  (set `self.LeftCorrect` false))

(event `RightDone`
  (set `self.RightCorrect` true)
  (if (`self.LeftCorrect`)
    (goto _label)))

(event `RightUnDone`
  (set `self.RightCorrect` false))

(fn `UserConstructionScript`)