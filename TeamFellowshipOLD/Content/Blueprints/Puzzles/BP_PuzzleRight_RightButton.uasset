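; Interactable button for the right-hand puzzle that turns a BP_PuzzleRight a quarter turn in pitch per press, while the linked bookcase's CanRotateRight is set.
; BeginPlay caches both level-assigned actors; each interaction disables rotation, animates the puzzle's scene through a timeline, then re-enables it.
; A wrapping four-step Direction counter on the puzzle triggers CorrectDirection at step 3, otherwise IncorrectDirection.
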(event `self.ReceiveBeginPlay`
  (bind _asbp_bookcase (cast `/Game/Blueprints/BP_Bookcase` (`self.Door_FromLevel`)))
  (set `self.BookcaseRef` _asbp_bookcase)
  (bind _asbp_puzzle_right (cast `/Game/Blueprints/Puzzles/BP_PuzzleRight` (`self.ActorFromLevel`)))
  (set `self.PuzzleRef` _asbp_puzzle_right))

(event `/Game/InteractableObjects/Interfaces/Interact.PossibleInteraction`
  (bind _puzzleref (`self.PuzzleRef`))
  (bind _puzzleref_2 (`self.PuzzleRef`))
  (bind _puzzleref_3 (`self.PuzzleRef`))
  (bind _pitch (`/Game/Blueprints/Puzzles/BP_PuzzleRight.Pitch` _puzzleref_2))
  (if (`/Game/Blueprints/BP_Bookcase.CanRotateRight` (`self.BookcaseRef`))
    (`/Game/Blueprints/Puzzles/BP_PuzzleRight.ToggleCanRotate` (`self.PuzzleRef`) false)
    (bind (_direction _newtrack_0) (`Timeline|Timeline_0` :!via `PlayFromStart`)
      (:`Update`
        (bind (_returnvalue_roll _returnvalue_pitch) (`KismetMathLibrary.BreakRotator` (`KismetMathLibrary.RLerp` (`KismetMathLibrary.MakeRotator` 0.0 _pitch 90.0) (`KismetMathLibrary.MakeRotator` 0.0 (+ _pitch 90.0) 90.0) _newtrack_0)))
        (`SceneComponent.K2_SetRelativeRotation` (`/Game/Blueprints/Puzzles/BP_PuzzleRight.Scene` (`self.PuzzleRef`)) (`KismetMathLibrary.MakeRotator` 0.0 _returnvalue_pitch) false false))
      (:`Finished`
        (set `/Game/Blueprints/Puzzles/BP_PuzzleRight.Pitch` _returnvalue_pitch _puzzleref_2)
        (`/Game/Blueprints/Puzzles/BP_PuzzleRight.ToggleCanRotate` (`self.PuzzleRef`) true)
        (bind _output_get (set `/Game/Blueprints/Puzzles/BP_PuzzleRight.Direction` (+ (`/Game/Blueprints/Puzzles/BP_PuzzleRight.Direction` _puzzleref_3) 1) _puzzleref_3))
        (if (== _output_get 3)
          (`/Game/Blueprints/Puzzles/BP_PuzzleRight.CorrectDirection` _puzzleref)
          (else
            (`/Game/Blueprints/Puzzles/BP_PuzzleRight.IncorrectDirection` _puzzleref)))
        (if (> _output_get 3)
          (set `/Game/Blueprints/Puzzles/BP_PuzzleRight.Direction` 0 _puzzleref))))))

(fn `UserConstructionScript`)