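; Interactable left button for the left puzzle, rotating a BP_PuzzleLeft piece a quarter turn per press.
; It casts level references to the bookcase and puzzle, gates presses on the bookcase's CanRotateLeft, and toggles rotation availability through the puzzle around each turn.
; A timeline lerps the puzzle's pitch by -90 degrees, then decrements its Direction with wraparound and reports whether it reached the correct facing.
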(event `self.ReceiveBeginPlay`
  (bind _asbp_bookcase (cast `/Game/Blueprints/BP_Bookcase` (`self.Door_FromLevel`)))
  (set `self.BookcaseRef` _asbp_bookcase)
  (bind _asbp_puzzle_left (cast `/Game/Blueprints/Puzzles/BP_PuzzleLeft` (`self.ActorFromLevel`)))
  (set `self.PuzzleRef` _asbp_puzzle_left))

(event `/Game/InteractableObjects/Interfaces/Interact.PossibleInteraction`
  (bind _puzzleref (`self.PuzzleRef`))
  (bind _puzzleref_2 (`self.PuzzleRef`))
  (bind _puzzleref_3 (`self.PuzzleRef`))
  (bind _pitch (`/Game/Blueprints/Puzzles/BP_PuzzleLeft.Pitch` (`self.PuzzleRef`)))
  (if (`/Game/Blueprints/BP_Bookcase.CanRotateLeft` (`self.BookcaseRef`))
    (`/Game/Blueprints/Puzzles/BP_PuzzleLeft.ToggleCanRotateLeft` (`self.PuzzleRef`) false)
    (bind (_direction _newtrack_0) (`Timeline|Timeline_0` :!via `PlayFromStart`)
      (:`Update`
        (bind (_returnvalue_roll _returnvalue_pitch) (`KismetMathLibrary.BreakRotator` (`KismetMathLibrary.RLerp` (`KismetMathLibrary.MakeRotator` 0.0 _pitch) (`KismetMathLibrary.MakeRotator` 0.0 (+ _pitch -90.0)) _newtrack_0)))
        (`SceneComponent.K2_SetRelativeRotation` (`/Game/Blueprints/Puzzles/BP_PuzzleLeft.Scene` (`self.PuzzleRef`)) (`KismetMathLibrary.MakeRotator` 0.0 _returnvalue_pitch) false false))
      (:`Finished`
        (set `/Game/Blueprints/Puzzles/BP_PuzzleLeft.Pitch` _returnvalue_pitch _puzzleref_2)
        (`/Game/Blueprints/Puzzles/BP_PuzzleLeft.ToggleCanRotateLeft` _puzzleref_2 true)
        (bind _output_get (set `/Game/Blueprints/Puzzles/BP_PuzzleLeft.Direction` (- (`/Game/Blueprints/Puzzles/BP_PuzzleLeft.Direction` _puzzleref) 1) _puzzleref))
        (if (== _output_get 2)
          (`/Game/Blueprints/Puzzles/BP_PuzzleLeft.CorrectDirection` _puzzleref_3)
          (else
            (`/Game/Blueprints/Puzzles/BP_PuzzleLeft.IncorrectDirection` _puzzleref_3)))
        (if (< _output_get 0)
          (set `/Game/Blueprints/Puzzles/BP_PuzzleLeft.Direction` 3 _puzzleref_3))))))

(fn `UserConstructionScript`)