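; Placeholder left cabinet door that the player can swing open and closed, unless it is locked.
; On interaction, one of two timelines lerps the door's relative yaw 100 degrees from its saved rotation, opening or closing it.
; An IsMoving flag ignores input mid-swing, and IsOpen flips when each timeline finishes.
; SetName writes a locked or press-E prompt to the player's interact UI, using a player reference cached at BeginPlay.
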(event `self.ReceiveBeginPlay`
  (bind _asplayer_character (cast `/Game/PlayerCharacter` (`GameplayStatics.GetPlayerCharacter` 0)))
  (set `self.PlayerRef` _asplayer_character))

(event `/Game/InteractableObjects/Interfaces/Interact.PossibleInteraction`
  (bind _savedrot (`self.SavedRot`))
  (bind _savedrot_2 (`self.SavedRot`))
  (if (`self.IsLocked?`)
    _
    (elif (not (`self.IsMoving?`))
      (set `self.IsMoving?` true)
      (if (`self.IsOpen?`)
        (set `self.SavedRot` (`SceneComponent.RelativeRotation` (`self.Door`)))
        (bind (_direction _newtrack_0) (`Timeline|Timeline_1` :!via `PlayFromStart`)
          (:`Update`
            (`SceneComponent.K2_SetRelativeRotation` (`self.Door`) (`KismetMathLibrary.RLerp` _savedrot (`KismetMathLibrary.MakeRotator` (.roll _savedrot) (.pitch _savedrot) (- (.yaw _savedrot) 100.0)) _newtrack_0) false false))
          (:`Finished`
            (set `self.IsMoving?` false)
            (set `self.IsOpen?` false)))
        (else
          (set `self.SavedRot` (`SceneComponent.RelativeRotation` (`self.Door`)))
          (bind (_direction_2 _newtrack_0_2) (`Timeline|Timeline_0` :!via `PlayFromStart`)
            (:`Update`
              (`SceneComponent.K2_SetRelativeRotation` (`self.Door`) (`KismetMathLibrary.RLerp` _savedrot_2 (`KismetMathLibrary.MakeRotator` (.roll _savedrot_2) (.pitch _savedrot_2) (+ (.yaw _savedrot_2) 100.0)) _newtrack_0_2) false false))
            (:`Finished`
              (set `self.IsMoving?` false)
              (set `self.IsOpen?` true))))))))

(event `/Game/InteractableObjects/Interfaces/Interact.SetName`
  (if (`self.IsLocked?`)
    (`TextBlock.SetText` (`/Game/UI/InteractUI.UseText` (`/Game/PlayerCharacter.InteractUI` (`self.PlayerRef`))) "Locked")
    (else
      (`TextBlock.SetText` (`/Game/UI/InteractUI.UseText` (`/Game/PlayerCharacter.InteractUI` (`self.PlayerRef`))) "Press E to interact with Cabinet Door"))))

(fn `UserConstructionScript`)