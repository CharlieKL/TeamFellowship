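; Placeholder book interactable that the player can pick up for close examination.
; On BeginPlay it caches the PlayerCharacter reference.
; Interacting sends its mesh to the player's Examine component as a non-code-lock item, flags the player as in a usable and shows the mouse cursor.
; SetName writes the interaction prompt to the player's interact UI.
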(event `self.ReceiveBeginPlay`
  (bind _asplayer_character (cast `/Game/PlayerCharacter` (`GameplayStatics.GetPlayerCharacter` 0)))
  (set `self.PlayerRef` _asplayer_character))

(event `/Game/InteractableObjects/Interfaces/Interact.PossibleInteraction`
  (`KismetSystemLibrary.PrintString` "Interaction Possible: Book")
  (`/Game/Blueprints/Examine/BP_RenderObject.StartExamine` (`/Game/PlayerCharacter.Examine_Ref` (`self.PlayerRef`)) (`self.Mesh`) false)
  (set `/Game/PlayerCharacter.IsInUsable?` true (`self.PlayerRef`))
  (set `PlayerController.bShowMouseCursor` true (`GameplayStatics.GetPlayerController` 0)))

(event `/Game/InteractableObjects/Interfaces/Interact.SetName`
  (`TextBlock.SetText` (`/Game/UI/InteractUI.UseText` (`/Game/PlayerCharacter.InteractUI` (`self.PlayerRef`))) "Press E to interact with Book"))

(fn `UserConstructionScript`)