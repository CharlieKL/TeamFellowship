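; BP_Drawer1 is an interactable drawer that slides open and closed when the player uses it, unless it is locked.
; PossibleInteraction toggles IsOpen by lerping the Drawer component's relative location 90 units along Y with one of two timelines, ignoring input while IsMoving.
; SetName writes a locked or interact prompt to the player's InteractUI through a PlayerRef cached on BeginPlay.
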(event `/Game/InteractableObjects/Interfaces/Interact.PossibleInteraction`
  (bind _savedloc (`self.SavedLoc`))
  (bind _savedloc_2 (`self.SavedLoc`))
  (bind _returnvalue (- _savedloc_2 (0.0 90.0 0.0)))
  (bind _returnvalue_2 (+ _savedloc (0.0 90.0 0.0)))
  (if (`self.IsLocked?`)
    _
    (elif (not (`self.IsMoving?`))
      (set `self.IsMoving?` true)
      (if (`self.IsOpen?`)
        (bind (_direction _newtrack_1) (`Timeline|Timeline_1` :!via `PlayFromStart`)
          (:`Update`
            (`SceneComponent.K2_SetRelativeLocation` (`self.Drawer`) (`KismetMathLibrary.VLerp` _savedloc _returnvalue_2 _newtrack_1) false false))
          (:`Finished`
            (set `self.SavedLoc` _returnvalue_2)
            (set `self.IsOpen?` false)
            (set `self.IsMoving?` false)))
        (else
          (set `self.SavedLoc` (`SceneComponent.RelativeLocation` (`self.Drawer`)))
          (bind (_direction_2 _newtrack_1_2) (`Timeline|Timeline_0` :!via `PlayFromStart`)
            (:`Update`
              (`SceneComponent.K2_SetRelativeLocation` (`self.Drawer`) (`KismetMathLibrary.VLerp` _savedloc_2 _returnvalue _newtrack_1_2) false false))
            (:`Finished`
              (set `self.SavedLoc` _returnvalue)
              (set `self.IsOpen?` true)
              (set `self.IsMoving?` false))))))))

(event `/Game/InteractableObjects/Interfaces/Interact.SetName`
  (bind _usetext (`/Game/UI/InteractUI.UseText` (`/Game/PlayerCharacter.InteractUI` (`self.PlayerRef`))))
  (if (`self.IsLocked?`)
    (`TextBlock.SetText` _usetext "Locked")
    (else
      (`TextBlock.SetText` _usetext "Press E to Interact with Drawer"))))

(event `self.ReceiveBeginPlay`
  (bind _asplayer_character (cast `/Game/PlayerCharacter` (`GameplayStatics.GetPlayerCharacter` 0)))
  (set `self.PlayerRef` _asplayer_character))

(fn `UserConstructionScript`)