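; Interactable cauldron puzzle that takes four held items in a fixed order.
; PossibleInteraction checks the player's held item against the next expected ingredient, drops it either way, and clears progress flags on a mistake.
; The fourth correct item triggers CorrectRecipe, which slides the Cube component along negative X with a timeline, and locks further interaction.
; SetName updates the player's interact prompt, blanking it once complete.
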(event `self.ReceiveBeginPlay`
  (bind _asplayer_character (cast `/Game/PlayerCharacter` (`GameplayStatics.GetPlayerCharacter` 0)))
  (set `self.PlayerRef` _asplayer_character))

(event `/Game/InteractableObjects/Interfaces/Interact.SetName`
  (bind _usetext (`/Game/UI/InteractUI.UseText` (`/Game/PlayerCharacter.InteractUI` (`self.PlayerRef`))))
  (if (`self.InteractionComplete`)
    (`TextBlock.SetText` _usetext "")
    (else
      (`TextBlock.SetText` _usetext "Press E to interact with Cauldron"))))

(event `/Game/InteractableObjects/Interfaces/Interact.PossibleInteraction`
  (if (`self.InteractionComplete`)
    _
    (elif (`/Game/PlayerCharacter.IsHoldingItem` (`self.PlayerRef`))
      (if (`self.Ingredient1Added`)
        (if (`self.Ingredient2Added`)
          (if (`self.Ingredient3Added`)
            (if (`KismetTextLibrary.EqualEqual_TextText` (`/Game/PlayerCharacter.HeldItem` (`self.PlayerRef`)) (`self.Item4`))
              (`/Game/PlayerCharacter.DropItem` (`self.PlayerRef`))
              (`KismetSystemLibrary.PrintString` "Correct Item")
              (`self.CorrectRecipe`)
              (set `self.InteractionComplete` true)
              (else
                (`KismetSystemLibrary.PrintString` "Wrong Item")
                (set `self.Ingredient1Added` false)
                (set `self.Ingredient2Added` false)
                (set `self.Ingredient3Added` false)
                (`/Game/PlayerCharacter.DropItem` (`self.PlayerRef`))))
            (elif (`KismetTextLibrary.EqualEqual_TextText` (`/Game/PlayerCharacter.HeldItem` (`self.PlayerRef`)) (`self.Item3`))
              (set `self.Ingredient3Added` true)
              (`/Game/PlayerCharacter.DropItem` (`self.PlayerRef`))
              (`KismetSystemLibrary.PrintString` "Correct Item")
              (else
                (`KismetSystemLibrary.PrintString` "Wrong Item")
                (set `self.Ingredient1Added` false)
                (set `self.Ingredient2Added` false)
                (set `self.Ingredient3Added` false)
                (`/Game/PlayerCharacter.DropItem` (`self.PlayerRef`)))))
          (elif (`KismetTextLibrary.EqualEqual_TextText` (`/Game/PlayerCharacter.HeldItem` (`self.PlayerRef`)) (`self.Item2`))
            (set `self.Ingredient2Added` true)
            (`/Game/PlayerCharacter.DropItem` (`self.PlayerRef`))
            (`KismetSystemLibrary.PrintString` "Correct Item")
            (else
              (`KismetSystemLibrary.PrintString` "Wrong Item")
              (set `self.Ingredient1Added` false)
              (set `self.Ingredient2Added` false)
              (`/Game/PlayerCharacter.DropItem` (`self.PlayerRef`)))))
        (elif (`KismetTextLibrary.EqualEqual_TextText` (`/Game/PlayerCharacter.HeldItem` (`self.PlayerRef`)) (`self.Item1`))
          (set `self.Ingredient1Added` true)
          (`/Game/PlayerCharacter.DropItem` (`self.PlayerRef`))
          (`KismetSystemLibrary.PrintString` "Correct Item")
          (else
            (`KismetSystemLibrary.PrintString` "Wrong Item")
            (set `self.Ingredient1Added` false)
            (`/Game/PlayerCharacter.DropItem` (`self.PlayerRef`))))))))

(event `CorrectRecipe`
  (bind _savedloc (`self.SavedLoc`))
  (bind _returnvalue (- _savedloc (90.0 0.0 0.0)))
  (set `self.SavedLoc` (`SceneComponent.RelativeLocation` (`self.Cube`)))
  (bind (_direction _newtrack_0) (`Timeline|Timeline_0` :!via `PlayFromStart`)
    (:`Update`
      (`SceneComponent.K2_SetRelativeLocation` (`self.Cube`) (`KismetMathLibrary.VLerp` _savedloc _returnvalue _newtrack_0) false false))
    (:`Finished`
      (set `self.SavedLoc` _returnvalue)
      (`KismetSystemLibrary.PrintString` "Hello"))))

(fn `UserConstructionScript`)