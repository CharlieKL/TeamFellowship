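; BP_LightSwitch is an interactable switch that toggles the main room lights and swaps a poster between plain and glowing looks.
; On BeginPlay it casts a level-assigned reference to BP_MainRoomLights and caches it.
; Each PossibleInteraction event flips IsLightOn and sets the light components' visibility, showing the emissive poster material when they are hidden.
; The flag reads inverted: IsLightOn becomes true when the lights are hidden.
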(event `self.ReceiveBeginPlay`
  (bind _asbp_main_room_lights (cast `/Game/Blueprints/Lights/BP_MainRoomLights` (`self.Light_FromLevel`)))
  (set `self.LightRef` _asbp_main_room_lights))

(event `/Game/InteractableObjects/Interfaces/Interact.PossibleInteraction`
  (if (`self.IsLightOn`)
    (`SceneComponent.SetVisibility` (`/Game/Blueprints/Lights/BP_MainRoomLights.MainRoom_Light_Back` (`self.LightRef`)) true false)
    (`SceneComponent.SetVisibility` (`/Game/Blueprints/Lights/BP_MainRoomLights.MainRoom_Light` (`self.LightRef`)) true false)
    (`SceneComponent.SetVisibility` (`/Game/Blueprints/Lights/BP_MainRoomLights.MainRoom_Light_Back` (`self.LightRef`)) true false)
    (set `self.IsLightOn` false)
    (`PrimitiveComponent.SetMaterial` (`StaticMeshActor.StaticMeshComponent` (`self.Poster_FromLevel`)) 0 "/Game/Meshes/Poster/Poster_NoEmissive_Mat.Poster_NoEmissive_Mat")
    (else
      (`SceneComponent.SetVisibility` (`/Game/Blueprints/Lights/BP_MainRoomLights.MainRoom_Light_Back` (`self.LightRef`)) false false)
      (`SceneComponent.SetVisibility` (`/Game/Blueprints/Lights/BP_MainRoomLights.MainRoom_Light` (`self.LightRef`)) false false)
      (`SceneComponent.SetVisibility` (`/Game/Blueprints/Lights/BP_MainRoomLights.MainRoom_Light_Back` (`self.LightRef`)) false false)
      (set `self.IsLightOn` true)
      (`PrimitiveComponent.SetMaterial` (`StaticMeshActor.StaticMeshComponent` (`self.Poster_FromLevel`)) 0 "/Game/Meshes/Poster/Poster_Emissive_Mat.Poster_Emissive_Mat"))))

(fn `UserConstructionScript`)