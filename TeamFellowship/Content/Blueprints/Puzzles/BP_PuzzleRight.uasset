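; BP_PuzzleRight is the right-hand piece of a bookcase puzzle, reporting its state to a BP_Bookcase door.
; On BeginPlay it casts a level-assigned door reference to BP_Bookcase and caches it.
; Its events forward correct or incorrect direction as RightDone or RightUndone calls, and pass a rotation toggle into the bookcase's CanRotateRight flag.
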(event `self.ReceiveBeginPlay`
  (bind _asbp_bookcase (cast `/Game/Blueprints/BP_Bookcase` (`self.Door_FromLevel`)))
  (set `self.BookcaseRef` _asbp_bookcase))

(event `CorrectDirection`
  (`/Game/Blueprints/BP_Bookcase.RightDone` (`self.BookcaseRef`)))

(event `IncorrectDirection`
  (`/Game/Blueprints/BP_Bookcase.RightUndone` (`self.BookcaseRef`)))

(event `ToggleCanRotate`
  (params (Bool :type Boolean))
  (set `/Game/Blueprints/BP_Bookcase.CanRotateRight` Bool (`self.BookcaseRef`)))

(fn `UserConstructionScript`)