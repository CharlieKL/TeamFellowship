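; BP_Riddle is an interactable lock puzzle prop that flies up to the player for inspection and returns afterward.
; Starting interaction saves its transform, flags the player as using it, and timeline-lerps its root to the player's Scene component before enabling the cursor and Game-and-UI input.
; Ending interaction lerps it back, hides the cursor and restores game-only input.
; It also sets the lock's use prompt and stores a UI reference.
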(event `self.ReceiveBeginPlay`
  (bind _asplayer_character (cast `/Game/PlayerCharacter` (`GameplayStatics.GetPlayerCharacter` 0)))
  (set `self.PlayerRef` _asplayer_character))

(event `EndInteraction`
  (bind _defaultsceneroot (`self.DefaultSceneRoot`))
  (set `PlayerController.bShowMouseCursor` false (`GameplayStatics.GetPlayerController` 0))
  (set `self.SavedLocEnd` (`SceneComponent.K2_GetComponentLocation` _defaultsceneroot))
  (set `self.SavedRotEnd` (`SceneComponent.K2_GetComponentRotation` _defaultsceneroot))
  (bind (_direction _newtrack_0) (`Timeline|Timeline_7` :!via `PlayFromStart`)
    (:`Update`
      (`SceneComponent.K2_SetWorldLocationAndRotation` (`self.DefaultSceneRoot`) (`KismetMathLibrary.VLerp` (`self.SavedLocEnd`) (`self.SavedLoc`) _newtrack_0) (`KismetMathLibrary.RLerp` (`self.SavedRotEnd`) (`self.SaveRot`) _newtrack_0) false false))
    (:`Finished`
      (set `/Game/PlayerCharacter.IsInUsable?` false (`self.PlayerRef`))
      (`WidgetBlueprintLibrary.SetInputMode_GameOnly` (`GameplayStatics.GetPlayerController` 0)))))

(event `/Game/InteractableObjects/Interfaces/Interact.PossibleInteraction`
  (bind _defaultsceneroot (`self.DefaultSceneRoot`))
  (set `self.SavedLoc` (`SceneComponent.K2_GetComponentLocation` _defaultsceneroot))
  (set `self.SaveRot` (`SceneComponent.K2_GetComponentRotation` _defaultsceneroot))
  (bind _asplayer_character (cast `/Game/PlayerCharacter` (`GameplayStatics.GetPlayerCharacter` 0)))
  (set `self.PlayerRef` _asplayer_character)
  (set `/Game/PlayerCharacter.IsInUsable?` true _asplayer_character)
  (bind (_direction _newtrack_0) (`Timeline|Timeline_6` :!via `PlayFromStart`)
    (:`Update`
      (bind _scene (`/Game/PlayerCharacter.Scene` _asplayer_character))
      (`SceneComponent.K2_SetWorldLocationAndRotation` (`self.DefaultSceneRoot`) (`KismetMathLibrary.VLerp` (`self.SavedLoc`) (`SceneComponent.K2_GetComponentLocation` _scene) _newtrack_0) (`KismetMathLibrary.RLerp` (`self.SaveRot`) (`SceneComponent.K2_GetComponentRotation` _scene) _newtrack_0 true) false false))
    (:`Finished`
      (set `PlayerController.bShowMouseCursor` true (`GameplayStatics.GetPlayerController` 0))
      (`WidgetBlueprintLibrary.SetInputMode_GameAndUIEx` (`GameplayStatics.GetPlayerController` 0) null))))

(event `/Game/InteractableObjects/Interfaces/Interact.SetName`
  (`TextBlock.SetText` (`/Game/UI/InteractUI.UseText` (`/Game/PlayerCharacter.InteractUI` (`self.PlayerRef`))) "Press E to interact with Lock"))

(event `GetRef`
  (params (Ref :type "/Game/Blueprints/Puzzles/Lock/DeskLockUI Object Reference"))
  (set `self.UIRef` Ref))

(fn `UserConstructionScript`)