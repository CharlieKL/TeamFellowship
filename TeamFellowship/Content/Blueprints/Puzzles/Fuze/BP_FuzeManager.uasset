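; Manages a five-lever fuse puzzle, using lever and pin actors supplied from the level.
; SwitchOnFuse runs chained timelines that enable each lever and light its indicator in sequence.
; Lever up/down events adjust a Voltage total and rotate the pin by per-lever amounts, then check the combination.
; The check only prints Correct when levers 1, 3 and 5 are up, ignoring levers 2, 4 and Voltage, otherwise Incorrect.
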(event `self.ReceiveBeginPlay`
  (bind _asbp_pin (cast `/Game/Blueprints/Puzzles/Fuze/BP_Pin` (`self.Pin_FromLevel`)))
  (set `self.PinRef` _asbp_pin)
  (`|ExecutionSequence`
    (:`then_0`
      (bind _asbp_lever_placeholder (cast `/Game/Blueprints/BP_LeverPlaceholder` (`self.Lever1_FromLevel`)))
      (set `self.Lever1Ref` _asbp_lever_placeholder))
    (:`then_1`
      (bind _asbp_lever_placeholder_2 (cast `/Game/Blueprints/BP_LeverPlaceholder` (`self.Lever2_FromLevel`)))
      (set `self.Lever2Ref` _asbp_lever_placeholder_2))
    (:`then_2`
      (bind _asbp_lever_placeholder_3 (cast `/Game/Blueprints/BP_LeverPlaceholder` (`self.Lever3_FromLevel`)))
      (set `self.Lever3Ref` _asbp_lever_placeholder_3))
    (:`then_3`
      (bind _asbp_lever_placeholder_4 (cast `/Game/Blueprints/BP_LeverPlaceholder` (`self.Lever4_FromLevel`)))
      (set `self.Lever4Ref` _asbp_lever_placeholder_4))
    (:`then_4`
      (bind _asbp_lever_placeholder_5 (cast `/Game/Blueprints/BP_LeverPlaceholder` (`self.Lever5_FromLevel`)))
      (set `self.Lever5Ref` _asbp_lever_placeholder_5))))

(event `LeverUp`
  (params (LeverNum :type Integer))
  (switch `int` LeverNum
    (:`1`
      (set `self.Lever1_IsUp` true)
      (`self.Lever1`)
      (`/Game/Blueprints/Puzzles/Fuze/BP_Pin.AddRot` (`self.PinRef`) 50.0))
    (:`2`
      (set `self.Lever2_IsUp` true)
      (`self.Lever2`)
      (`/Game/Blueprints/Puzzles/Fuze/BP_Pin.AddRot` (`self.PinRef`) 40.0))
    (:`3`
      (set `self.Lever3_IsUp` true)
      (`self.Lever3`)
      (`/Game/Blueprints/Puzzles/Fuze/BP_Pin.AddRot` (`self.PinRef`) 25.0))
    (:`4`
      (set `self.Lever4_IsUp` true)
      (`self.Lever4`)
      (`/Game/Blueprints/Puzzles/Fuze/BP_Pin.AddRot` (`self.PinRef`) 30.0))
    (:`5`
      (set `self.Lever5_IsUp` true)
      (`self.Lever5`)
      (`/Game/Blueprints/Puzzles/Fuze/BP_Pin.AddRot` (`self.PinRef`) 35.0)))
  (`self.CheckCombo`))

(event `CheckCombo`
  (if (and (`self.Lever1_IsUp`) (`self.Lever3_IsUp`) (`self.Lever5_IsUp`))
    (`KismetSystemLibrary.PrintString` "Correct")
    (else
      (`KismetSystemLibrary.PrintString` "Incorrect"))))

(event `LeverDown`
  (params (LeverNum :type Integer))
  (switch `int` LeverNum
    (:`1`
      (set `self.Lever1_IsUp` false)
      (`self.Lever1`)
      (`/Game/Blueprints/Puzzles/Fuze/BP_Pin.SubRot` (`self.PinRef`) 50.0))
    (:`2`
      (set `self.Lever2_IsUp` false)
      (`self.Lever2`)
      (`/Game/Blueprints/Puzzles/Fuze/BP_Pin.SubRot` (`self.PinRef`) 40.0))
    (:`3`
      (set `self.Lever3_IsUp` false)
      (`self.Lever3`)
      (`/Game/Blueprints/Puzzles/Fuze/BP_Pin.SubRot` (`self.PinRef`) 25.0))
    (:`4`
      (set `self.Lever4_IsUp` false)
      (`self.Lever4`)
      (`/Game/Blueprints/Puzzles/Fuze/BP_Pin.SubRot` (`self.PinRef`) 30.0))
    (:`5`
      (set `self.Lever5_IsUp` false)
      (`self.Lever5`)
      (`/Game/Blueprints/Puzzles/Fuze/BP_Pin.SubRot` (`self.PinRef`) 35.0)))
  (`self.CheckCombo`))

(event `SwitchOnFuse`
  (`Timeline|Timeline_0` :!via `PlayFromStart`
    (:`Finished`
      (set `/Game/Blueprints/BP_LeverPlaceholder.IsActive` true (`self.Lever1Ref`))
      (`PrimitiveComponent.SetMaterial` (`self.Light`) 0 "/Game/Placeholder/PlaceholderMeshes/Activated_MAT.Activated_MAT")
      (`Timeline|Timeline_4` :!via `PlayFromStart`
        (:`Finished`
          (set `/Game/Blueprints/BP_LeverPlaceholder.IsActive` true (`self.Lever2Ref`))
          (`PrimitiveComponent.SetMaterial` (`self.Light2`) 0 "/Game/Placeholder/PlaceholderMeshes/Activated_MAT.Activated_MAT")
          (`Timeline|Timeline_1` :!via `PlayFromStart`
            (:`Finished`
              (set `/Game/Blueprints/BP_LeverPlaceholder.IsActive` true (`self.Lever3Ref`))
              (`PrimitiveComponent.SetMaterial` (`self.Light3`) 0 "/Game/Placeholder/PlaceholderMeshes/Activated_MAT.Activated_MAT")
              (`Timeline|Timeline_2` :!via `PlayFromStart`
                (:`Finished`
                  (set `/Game/Blueprints/BP_LeverPlaceholder.IsActive` true (`self.Lever4Ref`))
                  (`PrimitiveComponent.SetMaterial` (`self.Light4`) 0 "/Game/Placeholder/PlaceholderMeshes/Activated_MAT.Activated_MAT")
                  (`Timeline|Timeline_3` :!via `PlayFromStart`
                    (:`Finished`
                      (set `/Game/Blueprints/BP_LeverPlaceholder.IsActive` true (`self.Lever5Ref`))
                      (`PrimitiveComponent.SetMaterial` (`self.Light5`) 0 "/Game/Placeholder/PlaceholderMeshes/Activated_MAT.Activated_MAT"))))))))))))

(event `Lever1`
  (if (`self.Lever1_IsUp`)
    (set `self.Voltage` (+ (`self.Voltage`) 10))
    (else
      (set `self.Voltage` (- (`self.Voltage`) 10)))))

(event `Lever2`
  (if (`self.Lever2_IsUp`)
    (set `self.Voltage` (+ (`self.Voltage`) 20))
    (else
      (set `self.Voltage` (- (`self.Voltage`) 20)))))

(event `Lever3`
  (if (`self.Lever3_IsUp`)
    (set `self.Voltage` (+ (`self.Voltage`) 30))
    (else
      (set `self.Voltage` (- (`self.Voltage`) 30)))))

(event `Lever4`
  (if (`self.Lever4_IsUp`)
    (set `self.Voltage` (+ (`self.Voltage`) 40))
    (else
      (set `self.Voltage` (- (`self.Voltage`) 40)))))

(event `Lever5`
  (if (`self.Lever5_IsUp`)
    (set `self.Voltage` (+ (`self.Voltage`) 50))
    (else
      (set `self.Voltage` (- (`self.Voltage`) 50)))))

(fn `UserConstructionScript`)