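; BP_Pin is a rotatable pin actor in the Fuze puzzle.
; AddRot and SubRot events step the stored CurrentRot up or down by a given amount and apply it as the Scene component's relative roll, with pitch and yaw held at zero.
; Each change prints the new rotation to screen for debugging, and the Blueprint itself holds no limits or solution check.
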(event `self.ReceiveBeginPlay`)

(event `AddRot`
  (params (Rot :type "Float (double-precision)"))
  (bind _returnvalue (+ (`self.CurrentRot`) Rot))
  (`SceneComponent.K2_SetRelativeRotation` (`self.Scene`) (`KismetMathLibrary.MakeRotator` _returnvalue) false false)
  (bind _output_get (set `self.CurrentRot` _returnvalue))
  (`KismetSystemLibrary.PrintString` (`KismetStringLibrary.Conv_DoubleToString` _output_get)))

(event `SubRot`
  (params (Rot :type "Float (double-precision)"))
  (bind _returnvalue (- (`self.CurrentRot`) Rot))
  (`SceneComponent.K2_SetRelativeRotation` (`self.Scene`) (`KismetMathLibrary.MakeRotator` _returnvalue) false false)
  (bind _output_get (set `self.CurrentRot` _returnvalue))
  (`KismetSystemLibrary.PrintString` (`KismetStringLibrary.Conv_DoubleToString` _output_get)))

(fn `UserConstructionScript`)