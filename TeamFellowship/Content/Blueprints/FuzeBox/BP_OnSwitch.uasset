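; BP_OnSwitch is a fuse box switch that the player activates by interacting while holding its required item.
; A matching item reveals the Switch component, and a timeline rotates it 90 degrees down in pitch from its current angle.
; When the animation finishes, it calls SwitchOnFuse on the level-referenced BP_FuzeManager and makes the player drop the held item.
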(event `self.ReceiveBeginPlay`
  (bind _asplayer_character (cast `/Game/PlayerCharacter` (`GameplayStatics.GetPlayerCharacter` 0)))
  (set `self.PlayerRef` _asplayer_character)
  (bind _asbp_fuze_manager (cast `/Game/Blueprints/Puzzles/Fuze/BP_FuzeManager` (`self.FuseManager_FromLevel`)))
  (set `self.FuseManagerRef` _asbp_fuze_manager))

(event `/Game/InteractableObjects/Interfaces/Interact.PossibleInteraction`
  (bind _switch (`self.Switch`))
  (bind _pitch (`self.Pitch`))
  (bind (_relativerotation_roll _relativerotation_pitch) (`KismetMathLibrary.BreakRotator` (`SceneComponent.RelativeRotation` _switch)))
  (if (`/Game/PlayerCharacter.IsHoldingItem` (`self.PlayerRef`))
    (if (`KismetTextLibrary.EqualEqual_TextText` (`/Game/PlayerCharacter.HeldItem` (`self.PlayerRef`)) (`self.Item`))
      (`SceneComponent.SetVisibility` (`self.Switch`) true false)
      (set `self.Pitch` _relativerotation_pitch)
      (bind (_direction _newtrack_0) (`Timeline|Timeline_0` :!via `PlayFromStart`)
        (:`Update`
          (bind (_returnvalue_roll _returnvalue_pitch) (`KismetMathLibrary.BreakRotator` (`KismetMathLibrary.RLerp` (`KismetMathLibrary.MakeRotator` 0.0 _pitch) (`KismetMathLibrary.MakeRotator` 0.0 (- _pitch 90.0)) _newtrack_0)))
          (`SceneComponent.K2_SetRelativeRotation` _switch (`KismetMathLibrary.MakeRotator` 0.0 _returnvalue_pitch) false false))
        (:`Finished`
          (`/Game/Blueprints/Puzzles/Fuze/BP_FuzeManager.SwitchOnFuse` (`self.FuseManagerRef`))
          (`/Game/PlayerCharacter.DropItem` (`self.PlayerRef`)))))))

(fn `UserConstructionScript`)