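; BP_RiddleBook is an interactable riddle book that opens in the player's examine view.
; On BeginPlay it caches a reference to the PlayerCharacter.
; PossibleInteraction starts an examination through the player's ExamineRef using the book's 3D model with the code lock flag off, sets IsInUsable on the player and shows the mouse cursor.
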(event `self.ReceiveBeginPlay`
  (bind _asplayer_character (cast `/Game/PlayerCharacter` (`GameplayStatics.GetPlayerCharacter` 0)))
  (set `self.PlayerRef` _asplayer_character))

(event `/Game/InteractableObjects/Interfaces/Interact.PossibleInteraction`
  (`/Game/Blueprints/Examine/BP_RenderObject.StartExamine` (`/Game/PlayerCharacter.Examine_Ref` (`self.PlayerRef`)) "/Game/Meshes/RiddleBook/Riddle_Book_3DModel.Riddle_Book_3DModel" false)
  (set `/Game/PlayerCharacter.IsInUsable?` true (`self.PlayerRef`))
  (set `PlayerController.bShowMouseCursor` true (`GameplayStatics.GetPlayerController` 0)))

(fn `UserConstructionScript`)