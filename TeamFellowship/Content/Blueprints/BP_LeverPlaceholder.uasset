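; BP_LeverPlaceholder is an interactable placeholder lever that reports its up or down state to a level-referenced BP_FuzeManager.
; BeginPlay casts the assigned manager reference and caches it.
; PossibleInteraction, gated by IsActive and IsMoving, snaps the Lever component's pitch back and forth by a fixed offset, flips IsUp, then calls LeverUp or LeverDown on the manager with its LeverNum.
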(event `self.ReceiveBeginPlay`
  (bind _asbp_fuze_manager (cast `/Game/Blueprints/Puzzles/Fuze/BP_FuzeManager` (`self.Manager_FromLevel`)))
  (set `self.ManagerRef` _asbp_fuze_manager))

(event `/Game/InteractableObjects/Interfaces/Interact.PossibleInteraction`
  (bind _savedrot (`self.SavedRot`))
  (bind _returnvalue (- _savedrot 100.0))
  (bind _returnvalue_2 (+ _savedrot 100.0))
  (if (`self.IsActive`)
    (if (`self.IsMoving`)
      _
      (elif (`self.IsUp`)
        (`SceneComponent.K2_SetRelativeRotation` (`self.Lever`) (`KismetMathLibrary.MakeRotator` 0.0 _returnvalue) false false)
        (set `self.SavedRot` _returnvalue)
        (set `self.IsUp` false)
        (`/Game/Blueprints/Puzzles/Fuze/BP_FuzeManager.LeverDown` (`self.ManagerRef`) (`self.LeverNum`))
        (else
          (`SceneComponent.K2_SetRelativeRotation` (`self.Lever`) (`KismetMathLibrary.MakeRotator` 0.0 _returnvalue_2) false false)
          (set `self.SavedRot` _returnvalue_2)
          (set `self.IsUp` true)
          (`/Game/Blueprints/Puzzles/Fuze/BP_FuzeManager.LeverUp` (`self.ManagerRef`) (`self.LeverNum`)))))))

(fn `UserConstructionScript`)