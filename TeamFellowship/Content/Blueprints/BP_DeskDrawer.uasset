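; BP_DeskDrawer is an interactable desk drawer that the player slides open or closed unless it is locked.
; Interaction toggles between two timelines that lerp the drawer's relative location along Y from its saved position, ignoring new input while moving.
; SetName updates the player's interact UI text to show either a locked notice or the key prompt.
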(event `self.ReceiveBeginPlay`
  (bind _asplayer_character (cast `/Game/PlayerCharacter` (`GameplayStatics.GetPlayerCharacter` 0)))
  (set `self.PlayerRef` _asplayer_character))

(event `/Game/InteractableObjects/Interfaces/Interact.PossibleInteraction`
  (bind _savedloc (`self.SavedLoc`))
  (bind _savedloc_2 (`self.SavedLoc`))
  (bind _returnvalue (- _savedloc (0.0 90.0 0.0)))
  (bind _returnvalue_2 (+ _savedloc_2 (0.0 90.0 0.0)))
  (if (`self.IsLocked?`)
    _
    (elif (not (`self.IsMoving?`))
      (set `self.IsMoving?` true)
      (if (`self.IsOpen?`)
        (set `self.SavedLoc` (`SceneComponent.RelativeLocation` (`self.DeskDrawer`)))
        (bind (_direction _newtrack_0) (`Timeline|Timeline_1` :!via `PlayFromStart`)
          (:`Update`
            (`SceneComponent.K2_SetRelativeLocation` (`self.DeskDrawer`) (`KismetMathLibrary.VLerp` _savedloc _returnvalue _newtrack_0) false false))
          (:`Finished`
            (set `self.SavedLoc` _returnvalue)
            (set `self.IsOpen?` false)
            (set `self.IsMoving?` false)))
        (else
          (set `self.SavedLoc` (`SceneComponent.RelativeLocation` (`self.DeskDrawer`)))
          (bind (_direction_2 _newtrack_0_2) (`Timeline|Timeline_0` :!via `PlayFromStart`)
            (:`Update`
              (`SceneComponent.K2_SetRelativeLocation` (`self.DeskDrawer`) (`KismetMathLibrary.VLerp` _savedloc_2 _returnvalue_2 _newtrack_0_2) false false))
            (:`Finished`
              (set `self.SavedLoc` _returnvalue_2)
              (set `self.IsOpen?` true)
              (set `self.IsMoving?` false))))))))

(event `/Game/InteractableObjects/Interfaces/Interact.SetName`
  (if (`self.IsLocked?`)
    (`TextBlock.SetText` (`/Game/UI/InteractUI.UseText` (`/Game/PlayerCharacter.InteractUI` (`self.PlayerRef`))) "Locked")
    (else
      (`TextBlock.SetText` (`/Game/UI/InteractUI.UseText` (`/Game/PlayerCharacter.InteractUI` (`self.PlayerRef`))) "Press E to interact with Drawer"))))

(fn `UserConstructionScript`)