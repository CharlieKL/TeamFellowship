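; BP_Bookcase is a puzzle-driven bookcase door that swings open once both its left and right conditions are correct.
; Done and Undone events set or clear a flag for each side, and each Done event prints a debug string, then calls OpenDoor if the other side is already correct.
; OpenDoor plays a timeline that lerps the Scene component's relative yaw 100 degrees down from SavedRot.
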(event `RightDone`
  (set `self.RightCorrect` true)
  (`KismetSystemLibrary.PrintString` "Hello")
  (if (`self.LeftCorrect`)
    (`self.OpenDoor` :!label _label)))

(event `RightUndone`
  (set `self.RightCorrect` false))

(event `LeftDone`
  (set `self.LeftCorrect` true)
  (`KismetSystemLibrary.PrintString` "Hello")
  (if (`self.RightCorrect`)
    (goto _label)))

(event `LeftUndone`
  (set `self.LeftCorrect` false))

(event `OpenDoor`
  (bind _savedrot (`self.SavedRot`))
  (bind (_direction _newtrack_0) (`Timeline|Timeline_0` :!via `PlayFromStart`)
    (:`Update`
      (bind (_returnvalue_roll _returnvalue_pitch _returnvalue_yaw) (`KismetMathLibrary.BreakRotator` (`KismetMathLibrary.RLerp` (`KismetMathLibrary.MakeRotator` 0.0 0.0 _savedrot) (`KismetMathLibrary.MakeRotator` 0.0 0.0 (- _savedrot 100.0)) _newtrack_0)))
      (`SceneComponent.K2_SetRelativeRotation` (`self.Scene`) (`KismetMathLibrary.MakeRotator` 0.0 0.0 _returnvalue_yaw) false false))))

(fn `UserConstructionScript`)