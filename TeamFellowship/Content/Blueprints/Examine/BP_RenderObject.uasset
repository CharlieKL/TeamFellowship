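; Actor that displays the mesh of the object the player examines in the examine UI.
; StartExamine resets the Cube component's world rotation and the stored rotation values, then swaps in the supplied mesh.
; It shows the player character's ExamineUI and switches input to UI-only with focus on that widget.
; The IsCodeLock parameter is unused, and nothing here applies the stored rotation or closes the view.
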(event `StartExamine`
  (params (NewMesh :type "StaticMesh Object Reference") (IsCodeLock :type Boolean))
  (`|ExecutionSequence`
    (:`then_0`
      (`SceneComponent.K2_SetWorldRotation` :`self` (`self.Cube`)))
    (:`then_1`
      (set `self.RotationX` 0.0))
    (:`then_2`
      (set `self.RotationY` 0.0))
    (:`then_3`
      (set `self.RotationZ` 0.0)
      (`StaticMeshComponent.SetStaticMesh` (`self.Cube`) NewMesh)
      (bind _asplayer_character (cast `/Game/PlayerCharacter` (`GameplayStatics.GetPlayerCharacter` 0)))
      (bind _examineui (`/Game/PlayerCharacter.ExamineUI` _asplayer_character))
      (`Widget.SetVisibility` _examineui "Visible")
      (`WidgetBlueprintLibrary.SetInputMode_UIOnlyEx` (`GameplayStatics.GetPlayerController` 0) _examineui))))

(fn `UserConstructionScript`)