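; BP_IngredientTest3 is a test ingredient that the player can pick up.
; On BeginPlay it caches the player character, cast to PlayerCharacter, in PlayerRef.
; PossibleInteraction passes its ItemName to the player's PickupItem, and SetName writes a fixed "Press E to pickup item" prompt to the player's interaction UI.
; The Blueprint itself does not hide or destroy the item after pickup.
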(event `self.ReceiveBeginPlay`
  (bind _asplayer_character (cast `/Game/PlayerCharacter` (`GameplayStatics.GetPlayerCharacter` 0)))
  (set `self.PlayerRef` _asplayer_character))

(event `/Game/InteractableObjects/Interfaces/Interact.PossibleInteraction`
  (`/Game/PlayerCharacter.PickupItem` (`self.PlayerRef`) (`self.ItemName`) null))

(event `/Game/InteractableObjects/Interfaces/Interact.SetName`
  (`TextBlock.SetText` (`/Game/UI/InteractUI.UseText` (`/Game/PlayerCharacter.InteractUI` (`self.PlayerRef`))) "Press E to pickup item"))

(fn `UserConstructionScript`)